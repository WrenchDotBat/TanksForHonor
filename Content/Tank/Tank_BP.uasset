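; Player-controlled tank Blueprint that drives by two tracks, orbits the camera rig and fires on the Shoot input.
; BeginPlay passes the Barrel and TankTurret components to setter functions, and Shoot calls Fire, with neither setters nor Fire defined here.
; Separate throttle axes feed each track, with the right value also printed.
; Azimuth and elevation axes rotate the Gimball and SpringArm, scaled by delta time for frame-rate independence.
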(event `self.ReceiveBeginPlay`
  (`self.SetBarrelRef` (`self.Barrel`))
  (`self.SetTurretRef` (`self.TankTurret`)))

(event `InputAxis|Right Throttle`
  (params (AxisValue :type "Float (single-precision)"))
  (`KismetSystemLibrary.PrintText` (`KismetTextLibrary.Conv_DoubleToText` AxisValue "HalfToEven"))
  (`TankTrack.SetThrottle` (`self.Right track`) AxisValue))

(event `InputAxis|Left Throttle`
  (params (AxisValue :type "Float (single-precision)"))
  (`TankTrack.SetThrottle` (`self.Left track`) AxisValue))

(event `InputAxis|AzimuthRotation`
  (params (AxisValue :type "Float (single-precision)"))
  (`SceneComponent.K2_AddLocalRotation` (`self.Gimball`) (`KismetMathLibrary.MakeRotator` 0.0 0.0 (* AxisValue (`GameplayStatics.GetWorldDeltaSeconds`) 100.0)) false false))

(event `InputAxis|Elevation`
  (params (AxisValue :type "Float (single-precision)"))
  (`SceneComponent.K2_AddLocalRotation` (`self.SpringArm`) (`KismetMathLibrary.MakeRotator` 0.0 (* AxisValue (`GameplayStatics.GetWorldDeltaSeconds`) 100.0)) false false))

(event `InputAction|Shoot`
  (params (Key :type "Key Structure"))
  (:`Pressed`
    (`self.Fire`)))

(fn `UserConstructionScript`)